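; BP_GameState is the game state that tracks how many speakers have been triggered and decides when the game is won.
; On BeginPlay it counts all BP_Speaker actors in the level and prints that total.
; RegisterSpeakerTriggered increments the triggered count and opens the GameWon level once it equals the total.
; An unconnected branch that would show a win widget never runs.
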(event EventBeginPlay
  (bind _outactors (Actor|GetAllActorsOfClass "/Game/Bleuprints/BP_Speaker.BP_Speaker_C"))
  (bind _output_get (Variables|Default|SetTotalSpeaker (Utilities|Array|Length _outactors)))
  (Development|PrintString (Utilities|String|ToString(Integer) _output_get)))

(event EventTick
  (params (DeltaSeconds :type Float%20%28single-precision%29)))

(fn ConstructionScript)

(fn RegisterSpeakerTriggered
  (bind _result (Math|Integer|IncrementInt (Variables|Default|GetTriggeredSpeaker))
    (:%20%20
      (Variables|Default|SetTriggeredSpeaker _result)
      (if (== (Variables|Default|GetTriggeredSpeaker) (Variables|Default|GetTotalSpeaker))
        (Game|OpenLevel(byObjectReference) "/Game/Levels/GameWon.GameWon")))))