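; GM_Game, by its name the game mode, scatters BP_Speaker actors across randomly chosen spawn points when play begins.
; SpawnSpeaker gathers all BP_Spawnpoint actors, then loops a fixed number of times, spawning a speaker at a random point's location with default rotation and scale.
; Each used point is removed from the local list and destroyed, so picks do not repeat.
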(event EventBeginPlay
  (CallFunction|SpawnSpeaker))

(event EventTick
  (params (DeltaSeconds :type Float%20%28single-precision%29)))

(fn ConstructionScript)

(fn SpawnSpeaker
  (bind _outactors (Actor|GetAllActorsOfClass "/Game/Bleuprints/BP_Spawnpoint.BP_Spawnpoint_C"))
  (LocalVariables|SetLocalSpawnReference _outactors)
  (for _index (range 0 3)
    (LocalVariables|SetLocalItem (.OutItem (Utilities|Array|Random (LocalVariables|GetLocalSpawnReference))))
    (Game|SpawnActorfromClass "/Game/Bleuprints/BP_Speaker.BP_Speaker_C" (Math|Transform|MakeTransform (Transformation|GetActorLocation (LocalVariables|GetLocalItem))) "AdjustIfPossibleButAlwaysSpawn" "MultiplyWithRoot" 0 0)
    (Utilities|Array|RemoveItem (LocalVariables|GetLocalSpawnReference) (LocalVariables|GetLocalItem))
    (Actor|DestroyActor (LocalVariables|GetLocalItem))))